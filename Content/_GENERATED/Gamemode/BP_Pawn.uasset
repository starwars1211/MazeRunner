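; BP_Pawn is a player pawn that fires hitscan shots from the camera on left mouse click.
; Each shot line-traces forward with debug drawing, damages the hit actor and spawns a BP_MyMasterField at the impact point.
; Single mode fires once per press, while Multy mode loops Shot on a fast timer until release.
; ChangeShotMode sets the mode, reverting Multy to Single after a retriggerable delay and clearing the timer.
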(event Custom|Shot
  (bind _returnvalue (Game|GetPlayerCameraManager 0))
  (bind _returnvalue_2 (Transformation|GetActorLocation _returnvalue))
  ;[1 1 1 1 20] 디폴트 폰 왼쪽 마우스를 누르면 트레이서가 10000거리까지 작동한다, 데미지는 1씩 들어간다
  (bind (_outhit _returnvalue_3) (Collision|LineTraceByChannel _returnvalue_2 (+ _returnvalue_2 (* (Math|Vector|GetForwardVector (Transformation|GetActorRotation _returnvalue)) 1e+04)) "TraceTypeQuery1" false 0 "ForDuration" true "(R=0.979167,G=0.000000,B=0.068294,A=1.000000)" "(R=0.234375,G=0.096780,B=0.008047,A=1.000000)"))
  (if _returnvalue_3
    (Game|Damage|ApplyDamage (.HitActor (Collision|BreakHitResult _outhit)) 1e+02 0 0)
    (Game|SpawnActorfromClass "/Game/BluePrint/BP_MyMasterField.BP_MyMasterField_C" (Math|Conversions|ToTransform(Vector) (.ImpactPoint (Collision|BreakHitResult _outhit))) "Undefined" "MultiplyWithRoot" 0 0)))

(event Custom|ChangeShotMode
  (params (NewParam :type E_ShotMode%20Enum :default "NewEnumerator0"))
  ;[1 1 1] 체인지샷모드가 되면 10초동안 실행하고 실글모드로 바꾸고 모드는 삭제
  (bind _output_get (Variables|Default|SetShotMode NewParam))
  (switch Utilities|FlowControl|Switch|SwitchonE_ShotMode _output_get
    (:NewEnumerator2
      (Utilities|FlowControl|RetriggerableDelay 1e+01)
      (Variables|Default|SetShotMode "NewEnumerator1")
      (Utilities|Time|ClearandInvalidateTimerbyHandle (Variables|Default|GetMultiShotHandle)))))

(event EventBeginPlay)

(event Collision|EventActorBeginOverlap
  (params (OtherActor :type Actor%20Object%20Reference)))

(event EventTick
  (params (DeltaSeconds :type Float%20%28single-precision%29)))

(event Input|MouseEvents|LeftMouseButton
  (params (Key :type Key%20Structure))
  ;[1 1 1] Comment
)

(event Input|MouseEvents|LeftMouseButton
  (params (Key :type Key%20Structure))
  (bind _shotmode (Variables|Default|GetShotMode))
  ;[1 1 1] 마우스를 왼쪽 버튼을 누르면싱글일땐 단발로 나가고 멀티일때는 0.005에한번씩(연사)가 멀티샷핸들동안 나간다
  (:Pressed
    (switch Utilities|FlowControl|Switch|SwitchonE_ShotMode _shotmode
      (:NewEnumerator1
        (CallFunction|Shot))
      (:NewEnumerator2
        (bind _returnvalue (Utilities|Time|SetTimerbyEvent (delegate Custom|Shot) 0.005 true))
        (Variables|Default|SetMultiShotHandle _returnvalue))))
  (:Released
    (switch Utilities|FlowControl|Switch|SwitchonE_ShotMode _shotmode
      (:NewEnumerator2
        (Utilities|Time|ClearandInvalidateTimerbyHandle (Variables|Default|GetMultiShotHandle))))))

(fn ConstructionScript)