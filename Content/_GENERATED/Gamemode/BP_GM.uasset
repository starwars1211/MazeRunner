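; Game mode for a timed target round: destroy every BP_Shpere before time runs out to win.
; BeginPlay counts the spheres and binds their OnDied dispatchers to a kill counter, while Tick runs the countdown and broadcasts it through Timepluse.
; Time and count sync with the game instance (BP_GI).
; A DoOnce-guarded Endgame pauses play, toggles UMG_MainUI's victory or defeat widgets, shows the cursor and submits the time as best time.
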(event Custom|Endgame
  (params (isVictory :type Boolean))
  ;[1 1 1 1 25] 게임이 끝나면 승리(VICTIRY) 또는 패배(DEFEAT)로 뜨는데 Do Once(한번만실행하라)를 이용해서 한번만 실행되게 된다
  (Utilities|FlowControl|DoOnce false
    (:Completed
      (Game|SetGamePaused true)
      (if isVictory
        (bind _array_element (CallFunction|UMGmainUIforEach))
        (Utilities|FlowControl|Sequence
          (:then_0
            (CallFunction|SetVisiblityMoniter (Variables|/Script/UMG.Widget|GetVisibility (Variables|/Game/_GENERATED/WBP/UMG_MainUI.UMG_MainUI_C|GetWGT_V _array_element)) (Variables|/Game/_GENERATED/WBP/UMG_MainUI.UMG_MainUI_C|GetWGT_V _array_element)))
          (:then_1
            (CallFunction|SetVisiblityMoniter (Variables|/Script/UMG.Widget|GetVisibility (Variables|/Game/_GENERATED/WBP/UMG_MainUI.UMG_MainUI_C|GetCanvasPanel_Result _array_element)) (Variables|/Game/_GENERATED/WBP/UMG_MainUI.UMG_MainUI_C|GetCanvasPanel_Result _array_element))))
        (else
          (bind _array_element_2 (CallFunction|UMGmainUIforEach))
          (Utilities|FlowControl|Sequence
            (:then_0
              (CallFunction|SetVisiblityMoniter (Variables|/Script/UMG.Widget|GetVisibility (Variables|/Game/_GENERATED/WBP/UMG_MainUI.UMG_MainUI_C|GetWGT_D _array_element_2)) (Variables|/Game/_GENERATED/WBP/UMG_MainUI.UMG_MainUI_C|GetWGT_D _array_element_2)))
            (:then_1
              (CallFunction|SetVisiblityMoniter (Variables|/Script/UMG.Widget|GetVisibility (Variables|/Game/_GENERATED/WBP/UMG_MainUI.UMG_MainUI_C|GetCanvasPanel_Result _array_element_2)) (Variables|/Game/_GENERATED/WBP/UMG_MainUI.UMG_MainUI_C|GetCanvasPanel_Result _array_element_2))))))
      (CallFunction|GameOverMoniter))))

(event Custom|OnDied_Event
  ;[1 1 1] 이벤트 디스패처
  (CallFunction|SphereTargetCount))

(event Custom|Timepluse_Event
  (params (Time :type Float%20%28double-precision%29))
  ;[1 1 1] 시간
  (bind _output_get (Variables|/Game/_GENERATED/Gamemode/BP_GI.BP_GI_C|SetTime (Variables|Default|GetAs%20BP%20GI) Time)))

(event Custom|GameOverMoniter
  (bind _returnvalue (Game|GetPlayerController 0))
  ;[1 1 1 1 30] 게임이 끝나면 마우스가 보이고 게임인스턴스로 타임을 보낸다
  (Input|SetInputModeGameOnly _returnvalue false)
  (Variables|/Script/Engine.PlayerController|SetbShowMouseCursor _returnvalue true)
  (bind _asbp_gi (Utilities|Casting|CastToBP_GI (Game|GetGameInstance)))
  (Default|SetBestTime _asbp_gi (Variables|Default|GetTime)))

(event EventBeginPlay
  ;[1 1 1 1 25] 게임시작시 시간은 Max값으로 하고 맵상의 BP스피어 Max개수를 보여준다
  (Utilities|FlowControl|Sequence
    (:then_0
      ;[1 1 1] Comment
      (bind _count (Class|IFGI|Getcount(Message) (Game|GetGameInstance)))
      (Variables|Default|SetTargetCount _count))
    (:then_1
      (Variables|Default|SetTime (Variables|Default|GetMaxTime))
      (bind _outactors (Actor|GetAllActorsOfClass "/Game/BluePrint/BP_Shpere.BP_Shpere_C"))
      (Variables|Default|SetMaxTarget (Utilities|Array|Length _outactors))
      ;[1 1 1] 이벤트 디스패처
      (for _array_element _outactors
        (EventDispatchers|AssignOnDied _array_element (delegate Custom|OnDied_Event))))
    (:then_2
      ;[1 1 1] 시간
      (bind _asbp_gi (Utilities|Casting|CastToBP_GI (Game|GetGameInstance)))
      (Variables|Default|SetAs%20BP%20GI _asbp_gi)
      (EventDispatchers|BindEventtoTimepluse (delegate Custom|Timepluse_Event))
      (Variables|Default|SetTime (stale Custom|Timepluse_Event _output_get)))))

(event EventTick
  (params (DeltaSeconds :type Float%20%28single-precision%29))
  ;[1 1 1 1 25] Tick 발생시마다 시간이 줄어들어 시간이 다되거나 타겟이 0이 되면 게임이 끝난다
  (if true
    (Utilities|FlowControl|Sequence
      (:then_0
        (bind _output_get (Variables|Default|SetTime (- (Variables|Default|GetTime) DeltaSeconds)))
        (bind _output_get_2 (Variables|/Game/_GENERATED/Gamemode/BP_GI.BP_GI_C|SetTime (Variables|Default|GetAs%20BP%20GI) _output_get))
        (Default|CallTimepluse _output_get_2)
        (if (<= _output_get 0.0)
          ;[1 1 1] 시간이 다 되면 게임이 끝남
          (CallFunction|Endgame false))))))

(fn ConstructionScript)

(fn SphereTargetCount
  ;[1 1 1 1 25] 타겟카운트하고 맥스값보다크거나 같으면 게임 끝난다,타겟카운트를 게임인스턴스로 전송
  (Utilities|FlowControl|Sequence
    (:then_0
      (bind _result (Math|Integer|IncrementInt (Variables|Default|GetTargetCount))
        (:%20%20
          (if (>= _result (Variables|Default|GetMaxTarget))
            (CallFunction|Endgame true)))))
    (:then_1
      (Class|IFGI|Setcount(Message) (Game|GetGameInstance) (Variables|Default|GetTargetCount) (Variables|Default|GetMaxTarget))
      (Utilities|Casting|CastToBP_GI (Game|GetGameInstance)))))

(fn UMGmainUIforEach
  (bind _foundwidgets (Widget|GetAllWidgetsOfClass "/Game/_GENERATED/WBP/UMG_MainUI.UMG_MainUI_C" true))
  (for _array_element _foundwidgets
    (return _array_element))
  (return _array_element))

(fn SetVisiblityMoniter
  (params (A :type ESlateVisibility%20Enum :default "Visible") (self2 :type Widget%20Object%20Reference))
  (Widget|SetVisibility self2 (select (Utilities|Enum|Equal(Enum) A "Hidden") "SelfHitTestInvisible" "Hidden")))

(fn Getcount
  (return 0 0))

(fn Interfaceprint
  (params (NewParam :type Integer))
  (return false))