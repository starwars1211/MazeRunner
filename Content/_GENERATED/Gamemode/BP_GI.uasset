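; Game instance that stores a count and persists the best time and player transform through save games.
; Init loads or creates the SG_Time save and always creates a fresh BP_SGP object without reading its slot.
; SetBestTime saves only higher values.
; Save and Load act only on an existing slot, with Save passing no object to write, while LoadActorAtTransform applies the held transform or creates the first save.
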(event Custom|SetBestTime
  (params (A :type Float%20%28double-precision%29))
  (bind _as_sg_time (Variables|Default|GetAs%20SG%20Time))
  ;[1 1 1 1 25] BestTime
  (if (> A (Variables|Default|GetBestTime))
    (bind _output_get (Variables|Default|SetBestTime A))
    (Variables|/Game/_GENERATED/SaveGame/SG_Time.SG_Time_C|SetBestTime _as_sg_time _output_get)
    (SaveGame|SaveGametoSlot _as_sg_time (Variables|/Game/_GENERATED/SaveGame/SG_Time.SG_Time_C|GetSlotName _as_sg_time) (Variables|/Game/_GENERATED/SaveGame/SG_Time.SG_Time_C|GetUserIndex _as_sg_time))))

(event Custom|Save
  (bind _bp_sgp_r (Variables|Default|GetBP%20SGP_R))
  (bind _bp_sgp_r_2 (Variables|Default|GetBP%20SGP_R))
  ;[1 1 1] 플레이어 세이브
  (bind _returnvalue (SaveGame|DoesSaveGameExist (Variables|/Game/_GENERATED/SaveGame/BP_SGP.BP_SGP_C|GetSlotName _bp_sgp_r_2) (Variables|/Game/_GENERATED/SaveGame/BP_SGP.BP_SGP_C|GetUserId _bp_sgp_r_2)))
  (if _returnvalue
    (Variables|/Game/_GENERATED/SaveGame/BP_SGP.BP_SGP_C|SetPlayerSave _bp_sgp_r (Transformation|GetActorTransform (Variables|Default|GetABP_PR)))
    (SaveGame|SaveGametoSlot 0 (Variables|/Game/_GENERATED/SaveGame/BP_SGP.BP_SGP_C|GetSlotName _bp_sgp_r) (Variables|/Game/_GENERATED/SaveGame/BP_SGP.BP_SGP_C|GetUserId _bp_sgp_r))))

(event Custom|Load
  (bind _bp_sgp_r (Variables|Default|GetBP%20SGP_R))
  ;[1 1 1] 플레이어 로드
  (bind _returnvalue (SaveGame|DoesSaveGameExist (Variables|/Game/_GENERATED/SaveGame/BP_SGP.BP_SGP_C|GetSlotName _bp_sgp_r) (Variables|/Game/_GENERATED/SaveGame/BP_SGP.BP_SGP_C|GetUserId _bp_sgp_r)))
  (if _returnvalue
    (Transformation|SetActorTransform (Variables|Default|GetABP_PR) (Variables|/Game/_GENERATED/SaveGame/BP_SGP.BP_SGP_C|GetPlayerSave (Variables|Default|GetBP%20SGP_R)))))

(event EventInit
  ;[1 1 1] 베스트 타임 저장
  (Utilities|FlowControl|Sequence
    (:then_0
      (bind _returnvalue (SaveGame|CreateSaveGameObject "/Game/_GENERATED/SaveGame/SG_Time.SG_Time_C"))
      (bind _returnvalue_2 (SaveGame|LoadGamefromSlot (Variables|/Game/_GENERATED/SaveGame/SG_Time.SG_Time_C|GetSlotName _returnvalue) (Variables|/Game/_GENERATED/SaveGame/SG_Time.SG_Time_C|GetUserIndex _returnvalue)))
      (bind _assg_time (Utilities|Casting|CastToSG_Time _returnvalue_2)
        (:then
          (bind _output_get (Variables|Default|SetAs%20SG%20Time _assg_time))
          (Variables|Default|SetBestTime (Variables|/Game/_GENERATED/SaveGame/SG_Time.SG_Time_C|GetBestTime _output_get)))
        (:CastFailed
          (Variables|Default|SetAs%20SG%20Time _returnvalue))))
    (:then_1
      ;[1 1 1] BP_SGP 레퍼런스 생성
      (bind _returnvalue_3 (SaveGame|CreateSaveGameObject "/Game/_GENERATED/SaveGame/BP_SGP.BP_SGP_C"))
      (Variables|Default|SetBP%20SGP_R _returnvalue_3))))

(event EventSetcount
  (params (Count :type Integer) (MaxCount :type Integer))
  ;[1 1 1] Count 받는다
  (Utilities|FlowControl|Sequence
    (:then_0
      (Variables|Default|SetCount Count))))

(fn LoadActoratTransform
  (bind _bp_sgp_r (Variables|Default|GetBP%20SGP_R))
  (bind _bp_sgp_r_2 (Variables|Default|GetBP%20SGP_R))
  ;[1 1 1 1 30] 세이브앤 로드
  ;;[1 1 1 1 25] 세이브파일유무 확인
  (bind _returnvalue (SaveGame|DoesSaveGameExist (Variables|/Game/_GENERATED/SaveGame/BP_SGP.BP_SGP_C|GetSlotName _bp_sgp_r) (Variables|/Game/_GENERATED/SaveGame/BP_SGP.BP_SGP_C|GetUserId _bp_sgp_r)))
  (if _returnvalue
    ;;[1 1 1 1 25] 세이브된 액터트랜스폼값을 적용
    (Transformation|SetActorTransform (Variables|Default|GetABP_PR) (Variables|/Game/_GENERATED/SaveGame/BP_SGP.BP_SGP_C|GetPlayerSave (Variables|Default|GetBP%20SGP_R)))
    (else
      ;;[1 1 1 1 25] 세이브클래스플레이어세이브에 플레이어트랜스폼변수를 저장한다
      (Variables|/Game/_GENERATED/SaveGame/BP_SGP.BP_SGP_C|SetPlayerSave _bp_sgp_r_2 (Transformation|GetActorTransform (Variables|Default|GetABP_PR)))
      (SaveGame|SaveGametoSlot _bp_sgp_r_2 (Variables|/Game/_GENERATED/SaveGame/BP_SGP.BP_SGP_C|GetSlotName _bp_sgp_r_2) (Variables|/Game/_GENERATED/SaveGame/BP_SGP.BP_SGP_C|GetUserId _bp_sgp_r_2)))))

(fn Fireget
  (return 0.0))

(fn Getcount
  (return (Variables|Default|GetCount) (Variables|Default|GetMaxCount)))

(fn Interfaceprint
  (params (NewParam :type Integer))
  (return false))