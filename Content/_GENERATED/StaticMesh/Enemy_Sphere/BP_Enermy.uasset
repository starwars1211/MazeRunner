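; Enemy actor that automatically fires bullets on a repeating timer.
; Tick accumulates delta time and, on reaching BulletTime, adds BulletSetCount to BulletCount and calls Fire.
; Fire spawns an explosion particle and a BP_Bullet at the Arrow component, calls Reset and zeroes the timer.
; An unconnected copy of the Fire logic and an unused explosion sound node remain.
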(event EventBeginPlay)

(event Collision|EventActorBeginOverlap
  (params (OtherActor :type Actor%20Object%20Reference)))

(event EventTick
  (params (DeltaSeconds :type Float%20%28single-precision%29))
  ;[1 1 1 1 25] 총알 나가는 이펙트
  (bind _output_get (Variables|Default|SetTime (+ (Variables|Default|GetTime) DeltaSeconds)))
  (if (>= _output_get (Variables|Default|GetBulletTime))
    (Variables|Default|SetBulletCount (+ (Variables|Default|GetBulletCount) (Variables|Default|GetBulletSetCount)))
    (CallFunction|Fire)))

(fn ConstructionScript)

(fn Fire
  ;[1 1 1 1 25] 이미터 발생하고 총알을 생성한다
  (if true
    (Effects|SpawnEmitteratLocation "/Game/StarterContent/Particles/P_Explosion.P_Explosion" (Transformation|GetWorldLocation (Variables|Default|GetArrow)))
    (Game|SpawnActorfromClass "/Game/_GENERATED/StaticMesh/Enemy_Sphere/BP_Bullet.BP_Bullet_C" (Transformation|GetWorldTransform (Variables|Default|GetArrow)) "Undefined" "MultiplyWithRoot" 0 0)
    (Class|TypedElementListLibrary|Reset)
    (Variables|Default|SetTime 0.0)))