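; BP_Enermy1 is an enemy actor that damages the player on overlap and bursts into flame.
; BeginPlay caches the player character and game instance; overlap with player 0 calls ChangeHP to subtract health, plays a 2D bubble sound and triggers FireFlame.
; FireFlame spawns a fire emitter at the Arrow component and destroys it after a delay.
; The timed fire on Tick and the end-overlap cleanup are disconnected, so neither runs.
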(event OnComponentEndOverlap(Arrow)
  (params (OverlappedComponent :type Primitive%20Component%20Object%20Reference) (OtherActor :type Actor%20Object%20Reference) (OtherComp :type Primitive%20Component%20Object%20Reference) (OtherBodyIndex :type Integer))
  ;[1 1 1 1 25] 파이어 이미터 없애는 노드
)

(event Custom|FireFlame
  ;[1 1 1 1 25] 파이어 생성후 제거
  ;;[1 1 1] 애로우위치에 이미터 생성
  (bind _returnvalue (Effects|SpawnEmitteratLocation "/Game/StarterContent/Particles/P_Fire.P_Fire" (Transformation|GetWorldLocation (Variables|Default|GetArrow))))
  (bind _output_get (Variables|Default|SetEmitterR _returnvalue))
  (Utilities|FlowControl|Delay 3.0)
  (Utilities|IsValid _output_get
    (:Is%20Valid
      ;;[1 1 1] 이미터를 제거한다
      (Components|DestroyComponent (Variables|Default|GetEmitterR))
      (Variables|Default|SetEmitterR 0)
      ;;[1 1 1] 타임 리셋
      (Variables|Default|SetTime1 0.0))))

(event EventBeginPlay
  ;[1 1 1 1 25] 게임인스턴스 플레이어 레퍼런스 가져오기 위한 노드
  (bind _asabp_player (Utilities|Casting|CastToABP_Player (Game|GetPlayerCharacter 0)))
  (Variables|Default|SetAs%20ABP%20Player _asabp_player)
  (bind _asbp_gi (Utilities|Casting|CastToBP_GI (Game|GetGameInstance)))
  (Variables|Default|SetAs%20BP%20GI _asbp_gi))

(event Collision|EventActorBeginOverlap
  (params (OtherActor :type Actor%20Object%20Reference))
  ;[1 1 1] 오버랩 되면 캐릭터 HP를 깎는다
  (if (== (Game|GetPlayerCharacter 0) OtherActor)
    (Default|ChangeHP (Variables|Default|GetAs%20ABP%20Player) 1e+01 false)
    (CallFunction|FireFlame)
    (Audio|PlaySound2D "/Game/_GENERATED/Audio/1814_water-bubbles-01.1814_water-bubbles-01" 1.0 1.0 0.0 0 0)))

(event EventTick
  (params (DeltaSeconds :type Float%20%28single-precision%29))
  ;[1 1 1 1 25] 5초 마다 1번씩 불을 뿜는다
)

(fn ConstructionScript
  (|CallParentFunction))

(fn Fireget
  (return 0.0))