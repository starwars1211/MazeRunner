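; BP_TriggerBox is a trigger actor that spawns a BP_Enermy1 at its Box location when the player first overlaps it.
; An IsSpawned flag, never cleared here, blocks later overlaps from spawning again.
; SetFire also sets a looping five-second timer to StartFire, which waits through a retriggerable delay, destroys any surviving spawn and calls SetFire again, continually replacing the enemy.
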(event Custom|SetFire
  ;[1 1 1 1 25] 5초 동안 BP에너미를 생성한다
  (bind _returnvalue (Utilities|Time|SetTimerbyEvent (delegate Custom|StartFire) 5.0 true))
  (Variables|Default|SetFireTimer _returnvalue)
  (bind _returnvalue_2 (Game|SpawnActorfromClass "/Game/_GENERATED/StaticMesh/Enemy_Sphere/BP_Enermy1.BP_Enermy1_C" (Math|Conversions|ToTransform(Vector) (Transformation|GetWorldLocation (Variables|Default|GetBox))) "Undefined" "MultiplyWithRoot" 0 0))
  (Variables|Default|SetSpawnedFire _returnvalue_2)
  ;;[1 1 1] 있을때 생성안되게
  (Variables|Default|SetIsSpawned true))

(event Custom|StartFire
  (bind _spawnedfire (Variables|Default|GetSpawnedFire))
  ;[1 1 1 1 25] 타이머후에 파이어가 있으면 파괴 후 다시 생성 없으면 다시 생성
  (Utilities|FlowControl|RetriggerableDelay 1.0)
  (Utilities|IsValid _spawnedfire
    (:Is%20Valid
      (Actor|DestroyActor _spawnedfire)
      (CallFunction|SetFire))
    (:Is%20Not%20Valid
      (CallFunction|SetFire))))

(event Collision|EventActorBeginOverlap
  (params (OtherActor :type Actor%20Object%20Reference))
  ;[1 1 1 1 25] 오버랩되면 셋파이어를 실행한다
  (Utilities|Casting|CastToABP_Player OtherActor)
  (if (not (Variables|Default|GetIsSpawned))
    (CallFunction|SetFire)))

(fn ConstructionScript)