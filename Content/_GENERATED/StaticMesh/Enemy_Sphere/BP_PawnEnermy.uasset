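; Sphere enemy pawn that costs the player HP and plays a bubble sound on overlap, and destroys itself when damage depletes its own HP.
; BeginPlay links its HP widget to itself, starts movement and caches the player reference.
; A timeline moves the sphere with sweep, and a FlipFlop alternates Reverse and Play on blocking hits.
; An older trigger-driven timeline movement remains disconnected and never runs.
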(event OnComponentBeginOverlap(Sphere1)
  (params (OverlappedComponent :type Primitive%20Component%20Object%20Reference) (OtherActor :type Actor%20Object%20Reference) (OtherComp :type Primitive%20Component%20Object%20Reference) (OtherBodyIndex :type Integer) (bFromSweep :type Boolean) (SweepResult :type Hit%20Result%20Structure%20%28by%20ref%29))
  ;[1 1 1 1 25] 폰이랑 오버랩 되면 HP가 마이너스 10 되게 하는 노드
  (if (== (Game|GetPlayerCharacter 0) OtherActor)
    (Default|ChangeHP (Variables|Default|GetAs%20ABP%20Player) 1e+01 false)
    (Audio|PlaySound2D "/Game/_GENERATED/Audio/1814_water-bubbles-01.1814_water-bubbles-01" 1.0 1.0 0.0 0 0)))

(event Custom|MoveRoof
  ;[1 1 1 1 25] 스피어 타임라인을 이용한  무브먼트(콜리전이 발생하면 리버스로 반환한다)
  (bind _새_트랙_1 (Timeline|스피어무브먼트위아래 Play)
    (:Update
      (bind _sweephitresult (Transformation|SetRelativeLocationAndRotation (Variables|Default|GetSphere) (Math|Vector|Lerp(Vector) _새_트랙_1 "0, 0, 0" 0.0) "0, 0, 0" true false))
      (if (.bBlockingHit (Collision|BreakHitResult _sweephitresult))
        (Utilities|FlowControl|FlipFlop
          (:A
            (Timeline|스피어무브먼트위아래 Reverse))
          (:B
            (Timeline|스피어무브먼트위아래 Play)))))))

(event EventBeginPlay
  ;[1 1 1] 게임 시작시 시퀀스 연결
  (Utilities|FlowControl|Sequence
    (:then_0
      ;[1 1 1 1 40] 스피어 HP 관련 노드
      ;;[1 1 1 1 30] 에너미HP위젯에 폰레퍼런스를 쓴다
      (bind _aswbp_enermy_hp (Utilities|Casting|CastToWBP_EnermyHP (UserInterface|GetUserWidgetObject (Variables|Default|GetHp))))
      (Default|SetEnermy _aswbp_enermy_hp self))
    (:then_1
      ;[1 1 1] 무브루프이벤트 실행
      (CallFunction|MoveRoof))
    (:then_2
      ;[1 1 1 1 25] 플레이어 레퍼런스를 불러온다
      (bind _asabp_player (Utilities|Casting|CastToABP_Player (Game|GetPlayerCharacter 0)))
      (Variables|Default|SetAs%20ABP%20Player _asabp_player))))

(event Collision|EventActorBeginOverlap
  (params (OtherActor :type Actor%20Object%20Reference)))

(event EventTick
  (params (DeltaSeconds :type Float%20%28single-precision%29)))

(event Game|Damage|EventAnyDamage
  (params (Damage :type Float%20%28single-precision%29) (DamageType :type Damage%20Type%20Object%20Reference) (InstigatedBy :type Controller%20Object%20Reference) (DamageCauser :type Actor%20Object%20Reference))
  ;[1 1 1 1 40] 스피어 HP 관련 노드
  ;;[1 1 1 1 30] 데미지를 받아서 0이 되게 되면 사라지게 된다
  (bind _output_get (Variables|Default|SetPawnEnermyHp (- (Variables|Default|GetPawnEnermyHp) Damage)))
  (if (<= _output_get 0.0)
    ;;;[1 1 1] 스피어 사라지게 한다
    (Actor|DestroyActor)))

(fn ConstructionScript)