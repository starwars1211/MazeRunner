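; Enemy sphere actor that takes damage, shows its energy on a bar widget and explodes at zero.
; BeginPlay caches the Energebar widget from the EnermyHp component, and AnyDamage updates its percentage.
; At zero, Die spawns an explosion, fires the OnDied dispatcher and destroys the actor, and AnyDamage plays a sound.
; Hit, EndPlay and interface events are empty, and the game-mode target-count call is disconnected.
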(event OnComponentHit(Sphere)
  (params (HitComponent :type Primitive%20Component%20Object%20Reference) (OtherActor :type Actor%20Object%20Reference) (OtherComp :type Primitive%20Component%20Object%20Reference) (NormalImpulse :type Vector :default "0, 0, 0") (Hit :type Hit%20Result%20Structure%20%28by%20ref%29)))

(event Custom|Die
  ;[1 1 1 1 25] 로케이션에 있는 액터가 파괴되면 콜을 준다.
  (Effects|SpawnEmitteratLocation "/Game/StarterContent/Particles/P_Explosion.P_Explosion" (Transformation|GetActorLocation))
  (Default|CallOnDied)
  (Actor|DestroyActor))

(event EventBeginPlay
  ;[1 1 1] BP스피어 에너지바 위젯 연결 노드
  (Utilities|FlowControl|Sequence
    (:then_0
      (bind _asenergebar (Utilities|Casting|CastToEnergebar (UserInterface|GetUserWidgetObject (Variables|Default|GetEnermyHp))))
      (bind _output_get (Variables|Default|SetAs%20Energebar _asenergebar))
      (Variables|/Game/_GENERATED/WBP/Energebar.Energebar_C|SetEnergyPercent _output_get (/ (Variables|Default|GetEnergy) (Variables|Default|GetinIt_Energy))))))

(event Collision|EventActorBeginOverlap
  (params (OtherActor :type Actor%20Object%20Reference)))

(event EventTick
  (params (DeltaSeconds :type Float%20%28single-precision%29)))

(event EventEndPlay
  (params (EndPlayReason :type EEndPlayReason%20Enum :default "Destroyed")))

(event EventInterfaceprint)

(event Game|Damage|EventAnyDamage
  (params (Damage :type Float%20%28single-precision%29) (DamageType :type Damage%20Type%20Object%20Reference) (InstigatedBy :type Controller%20Object%20Reference) (DamageCauser :type Actor%20Object%20Reference))
  ;[1 1 1 1 25] 데미지를 받으면 에너지바위젯에 Set을하고 에너지가 0이 되면  다이를 실행한다
  (Variables|Default|SetEnergy (- (Variables|Default|GetEnergy) Damage))
  (bind _output_get (Variables|/Game/_GENERATED/WBP/Energebar.Energebar_C|SetEnergyPercent (Variables|Default|GetAs%20Energebar) (/ (Variables|Default|GetEnergy) (Variables|Default|GetinIt_Energy))))
  (if (<= _output_get 0.0)
    (CallFunction|Die)
    (Audio|PlaySound2D "/Game/StarterContent/Audio/Explosion02.Explosion02" 1.0 1.0 0.0 0 0)))

(fn ConstructionScript)