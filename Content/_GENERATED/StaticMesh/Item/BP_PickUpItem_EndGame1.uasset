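; Pickup item that ends the game when it is picked up.
; On BeginPlay it casts the game mode to BP_GM and caches the reference; the parent BeginPlay call is disconnected.
; The PickedThisUp event plays a 2D applause sound and calls Endgame with true on that cached game mode.
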(event EventBeginPlay
  ;[1 1 1] 게임모드레퍼런스 불러오기
  (bind _asbp_gm (Utilities|Casting|CastToBP_GM (Game|GetGameMode)))
  (Variables|Default|SetAs%20BP%20GM_0 _asbp_gm))

(event Collision|EventActorBeginOverlap
  (params (OtherActor :type Actor%20Object%20Reference))
  (|CallParentFunction OtherActor) ; 지금 이 노드는 비활성 상태입니다. \n핀을 끌어서 다른 노드를 연결하면 활성화됩니다.
)

(event EventTick
  (params (DeltaSeconds :type Float%20%28single-precision%29))
  (|CallParentFunction DeltaSeconds) ; 지금 이 노드는 비활성 상태입니다. \n핀을 끌어서 다른 노드를 연결하면 활성화됩니다.
)

(event EventPickedThisUp
  (params (Other%20Actor :type Actor%20Object%20Reference))
  ;[1 1 1] 엔드게임
  (Audio|PlaySound2D "/Game/_GENERATED/Audio/1819_applause-02.1819_applause-02" 1.0 1.0 0.0 0 0)
  (Default|Endgame (Variables|Default|GetAs%20BP%20GM_0) true))

(fn ConstructionScript
  (|CallParentFunction))