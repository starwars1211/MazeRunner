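; BP_PickUpItem_Level3Chage1 is a pickup item child Blueprint that serves as a transition to level 3.
; Its PickedThisUp event opens GM_Level3 by name.
; Its Sphere1 begin-overlap handler calls the parent PickedThisUp, noted as making the item disappear, and plays a 2D applause sound without filtering the overlapping actor.
; BeginPlay, ActorBeginOverlap and Tick are disabled placeholders.
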(event OnComponentBeginOverlap(Sphere1)
  (params (OverlappedComponent :type Primitive%20Component%20Object%20Reference) (OtherActor :type Actor%20Object%20Reference) (OtherComp :type Primitive%20Component%20Object%20Reference) (OtherBodyIndex :type Integer) (bFromSweep :type Boolean) (SweepResult :type Hit%20Result%20Structure%20%28by%20ref%29))
  ;[1 1 1] 먹게되면 사라진다
  (|CallParentFunction 0)
  (Audio|PlaySound2D "/Game/_GENERATED/Audio/1819_applause-02.1819_applause-02" 1.0 1.0 0.0 0 0))

(event EventBeginPlay
  (|CallParentFunction) ; 지금 이 노드는 비활성 상태입니다. \n핀을 끌어서 다른 노드를 연결하면 활성화됩니다.
)

(event Collision|EventActorBeginOverlap
  (params (OtherActor :type Actor%20Object%20Reference))
  (|CallParentFunction OtherActor) ; 지금 이 노드는 비활성 상태입니다. \n핀을 끌어서 다른 노드를 연결하면 활성화됩니다.
)

(event EventTick
  (params (DeltaSeconds :type Float%20%28single-precision%29))
  (|CallParentFunction DeltaSeconds) ; 지금 이 노드는 비활성 상태입니다. \n핀을 끌어서 다른 노드를 연결하면 활성화됩니다.
)

(event EventPickedThisUp
  (params (Other%20Actor :type Actor%20Object%20Reference))
  ;[1 1 1] 3레벨로 이동한다
  (Game|OpenLevel(byName) "GM_Level3"))

(fn ConstructionScript
  (|CallParentFunction))