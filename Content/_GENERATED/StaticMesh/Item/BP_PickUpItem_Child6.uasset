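; Child pickup item, apparently of BP_PickUpItem, that raises the sphere count when picked up, then destroys itself.
; BeginPlay caches the BP_GM game mode without calling the parent's BeginPlay.
; Sphere1 overlap runs the parent's pickup logic, while the PickedThisUp override fires SphereUp and destroys the actor.
; SphereUp increases the game mode's TargetCount by a fixed step, clamped to a small range.
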(event OnComponentBeginOverlap(Sphere1)
  (params (OverlappedComponent :type Primitive%20Component%20Object%20Reference) (OtherActor :type Actor%20Object%20Reference) (OtherComp :type Primitive%20Component%20Object%20Reference) (OtherBodyIndex :type Integer) (bFromSweep :type Boolean) (SweepResult :type Hit%20Result%20Structure%20%28by%20ref%29))
  ;[1 1 1] 부모이벤트 똑같이 실행한다(예:사운드)
  (|CallParentFunction 0))

(event Custom|SphereUp
  ;[1 1 1] 아이템먹었을시 스피어 점수가 올라간다
  (Variables|/Game/BluePrint/Gamemode/BP_GM.BP_GM_C|SetTargetCount (Variables|Default|GetChangeCount) (Math|Integer|Clamp(Integer) (+ (Variables|/Game/BluePrint/Gamemode/BP_GM.BP_GM_C|GetTargetCount (Variables|Default|GetChangeCount)) 3) 1 5)))

(event EventBeginPlay
  ;[1 1 1] 비긴플레이에 연결 안됐을시 오류가 나서 이은 노드
  (bind _asbp_gm (Utilities|Casting|CastToBP_GM (Game|GetGameMode)))
  (Variables|Default|SetChangeCount _asbp_gm))

(event Collision|EventActorBeginOverlap
  (params (OtherActor :type Actor%20Object%20Reference))
  (|CallParentFunction OtherActor) ; This node is disabled and will not be called.\nDrag off pins to build functionality.
)

(event EventTick
  (params (DeltaSeconds :type Float%20%28single-precision%29))
  (|CallParentFunction DeltaSeconds) ; This node is disabled and will not be called.\nDrag off pins to build functionality.
)

(event EventPickedThisUp
  (params (Other%20Actor :type Actor%20Object%20Reference))
  ;[1 1 1] 픽업이벤트시 스피어업이벤트발생하고 이후 액터 파괴
  (CallFunction|SphereUp)
  (Actor|DestroyActor))

(fn ConstructionScript
  (|CallParentFunction))