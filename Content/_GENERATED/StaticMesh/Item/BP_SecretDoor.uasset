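; BP_SecretDoor is a secret door that opens when the player character enters its Box trigger and closes when they leave.
; Overlap begin plays the DoorOpenClose timeline and overlap end reverses it.
; Its OutoDoor track drives the Scene component's relative location through a vector lerp with Alpha fixed at zero, so the track value passes straight through.
; Disconnected nodes retain an unused scale-based door approach.
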(event OnComponentEndOverlap(Box)
  (params (OverlappedComponent :type Primitive%20Component%20Object%20Reference) (OtherActor :type Actor%20Object%20Reference) (OtherComp :type Primitive%20Component%20Object%20Reference) (OtherBodyIndex :type Integer))
  ;[1 1 1 1 30] 시크릿도어가 트리거박스 오버랩되면 문이 열리고 오버랩이 끝나면 문이 닫히는 노드
  (if (== (Game|GetPlayerCharacter 0) OtherActor)
    (bind _output_get (Variables|Default|SetCaractorinout false))
    (if (not _output_get)
      (bind _outodoor (Timeline|DoorOpenClose Reverse)
        (:Update
          (Transformation|SetRelativeLocationAndRotation (Variables|Default|GetScene) (Math|Vector|Lerp(Vector) _outodoor "0, 0, 0" 0.0) "0, 0, 0" false false))))))

(event OnComponentBeginOverlap(Box)
  (params (OverlappedComponent :type Primitive%20Component%20Object%20Reference) (OtherActor :type Actor%20Object%20Reference) (OtherComp :type Primitive%20Component%20Object%20Reference) (OtherBodyIndex :type Integer) (bFromSweep :type Boolean) (SweepResult :type Hit%20Result%20Structure%20%28by%20ref%29))
  ;[1 1 1 1 30] 시크릿도어가 트리거박스 오버랩되면 문이 열리고 오버랩이 끝나면 문이 닫히는 노드
  (if (== (Game|GetPlayerCharacter 0) OtherActor)
    (bind _output_get (Variables|Default|SetCaractorinout true))
    (if _output_get
      (bind _outodoor (Timeline|DoorOpenClose Play)
        (:Update
          (Transformation|SetRelativeLocationAndRotation (Variables|Default|GetScene) (Math|Vector|Lerp(Vector) _outodoor "0, 0, 0" 0.0) "0, 0, 0" false false))))))

(event EventBeginPlay)

(event Collision|EventActorBeginOverlap
  (params (OtherActor :type Actor%20Object%20Reference)))

(event EventTick
  (params (DeltaSeconds :type Float%20%28single-precision%29)))

(fn ConstructionScript)