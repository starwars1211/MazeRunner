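; A pickup item child Blueprint that switches the player's shot mode, noted as multi-shot, when picked up.
; PickedThisUp calls PickThis to play a 2D sound, destroys the actor, then casts player pawn 0 to BP_Pawn and calls ChangeShotMode.
; The mode change targets the player pawn regardless of OtherActor.
; The sphere overlap event here is empty, and the default events are disabled.
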(event OnComponentBeginOverlap(Sphere1)
  (params (OverlappedComponent :type Primitive%20Component%20Object%20Reference) (OtherActor :type Actor%20Object%20Reference) (OtherComp :type Primitive%20Component%20Object%20Reference) (OtherBodyIndex :type Integer) (bFromSweep :type Boolean) (SweepResult :type Hit%20Result%20Structure%20%28by%20ref%29)))

(event Custom|PickThis
  (params (OtherActor :type Actor%20Object%20Reference))
  ;[1 1 1] 먹었을때 사운드(사운드만 변경해주면 됨)
  (Audio|PlaySound2D (Variables|Default|GetSound) 1.0 1.0 0.0 0 0))

(event EventBeginPlay
  (|CallParentFunction) ; This node is disabled and will not be called.\nDrag off pins to build functionality.
)

(event Collision|EventActorBeginOverlap
  (params (OtherActor :type Actor%20Object%20Reference))
  (|CallParentFunction OtherActor) ; This node is disabled and will not be called.\nDrag off pins to build functionality.
)

(event EventTick
  (params (DeltaSeconds :type Float%20%28single-precision%29))
  (|CallParentFunction DeltaSeconds) ; This node is disabled and will not be called.\nDrag off pins to build functionality.
)

(event EventPickedThisUp
  (params (Other%20Actor :type Actor%20Object%20Reference))
  ;[1 1 1] 오버랩 되면 사운드 실행 액터 사라진후 BP폰에서 AsBPPawn실행되는동안ChangeShotMode멀티로바꿔주겠다는 노드
  (CallFunction|PickThis Other%20Actor)
  (Actor|DestroyActor)
  (bind _asbp_pawn (Utilities|Casting|CastToBP_Pawn (Game|Player|GetPlayerPawn 0)))
  (bind _output_get (Variables|Default|SetAs%20BP%20Pawn _asbp_pawn))
  (Default|ChangeShotMode _output_get "NewEnumerator2"))

(fn ConstructionScript
  (|CallParentFunction))