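; BP_PickUpItem_Child3 is a child pickup item that acts as a time penalty on the game timer.
; BeginPlay caches the BP_GM game mode without calling the parent's BeginPlay.
; The PickedThisUp override runs Time_Down, which cuts the game mode's Time by a fixed amount within clamped limits.
; Sphere1 overlap calls the parent PickedThisUp directly, noted as playing a sound and removing the item, with no actor filter.
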(event OnComponentBeginOverlap(Sphere1)
  (params (OverlappedComponent :type Primitive%20Component%20Object%20Reference) (OtherActor :type Actor%20Object%20Reference) (OtherComp :type Primitive%20Component%20Object%20Reference) (OtherBodyIndex :type Integer) (bFromSweep :type Boolean) (SweepResult :type Hit%20Result%20Structure%20%28by%20ref%29))
  ;[1 1 1 1 25] 소리가 나며 사라진다
  (|CallParentFunction 0))

(event Custom|Time_Down
  ;[1 1 1 1 25] 시간 줄어들게 하는 노드
  (Variables|/Game/BluePrint/Gamemode/BP_GM.BP_GM_C|SetTime (Variables|Default|GetBP_GMReference) (Math|Float|Clamp(Float) (- (Variables|/Game/BluePrint/Gamemode/BP_GM.BP_GM_C|GetTime (Variables|Default|GetBP_GMReference)) 1e+01) 1.0 6e+01)))

(event Collision|EventActorBeginOverlap
  (params (OtherActor :type Actor%20Object%20Reference))
  (|CallParentFunction OtherActor) ; This node is disabled and will not be called.\nDrag off pins to build functionality.
)

(event EventTick
  (params (DeltaSeconds :type Float%20%28single-precision%29))
  (|CallParentFunction DeltaSeconds) ; This node is disabled and will not be called.\nDrag off pins to build functionality.
)

(event EventPickedThisUp
  (params (Other%20Actor :type Actor%20Object%20Reference))
  ;[1 1 1 1 25] 시간 줄이는 이벤트 실행
  (CallFunction|TimeDown))

(event EventBeginPlay
  ;[1 1 1 1 25] 게임모드 레퍼런스를 가져오기 위한 노드
  (bind _asbp_gm (Utilities|Casting|CastToBP_GM (Game|GetGameMode)))
  (Variables|Default|SetBP_GMReference _asbp_gm))

(fn ConstructionScript
  (|CallParentFunction))