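; Child pickup item Blueprint that extends the game timer stored in BP_GM.
; BeginPlay caches the game mode cast to BP_GM for later use.
; Its PickedThisUp event calls TimeUp, which adds a fixed bonus to the game mode's Time, truncated to an integer and clamped to a set range.
; Sphere1 overlap calls the parent's PickedThisUp implementation rather than calling TimeUp directly.
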(event OnComponentBeginOverlap(Sphere1)
  (params (OverlappedComponent :type Primitive%20Component%20Object%20Reference) (OtherActor :type Actor%20Object%20Reference) (OtherComp :type Primitive%20Component%20Object%20Reference) (OtherBodyIndex :type Integer) (bFromSweep :type Boolean) (SweepResult :type Hit%20Result%20Structure%20%28by%20ref%29))
  ;[1 1 1 1 20] 부모가 가진 이벤트를 오버랩시 실행시킨다
  (|CallParentFunction 0))

(event Custom|TimeUp
  (params (NewParam :type Actor%20Object%20Reference))
  ;[1 1 1 1 25] 게임모드의 시간이 올라가야하니까 게임모드에서 시간을 더할 변수(Time) 가져와서 원하는 더하기 값을 클램프로 미니맥스값을 지정해주고 다시 타임값에 set(적용)한다    타임업 이벤트가 발생하면 실행된다. 이벤트비긴플레이에 연결이 안되어 있을시 실행 오류가 뜨니 연결에 주의하자
  (Variables|/Game/_GENERATED/Gamemode/BP_GM.BP_GM_C|SetTime (Variables|Default|GetBP_GMTime) (Math|Conversions|ToFloat(Integer) (Math|Integer|Clamp(Integer) (Math|Float|Truncate (+ (Variables|/Game/_GENERATED/Gamemode/BP_GM.BP_GM_C|GetTime (Variables|Default|GetBP_GMTime)) 1e+01)) 1 60))))

(event Collision|EventActorBeginOverlap
  (params (OtherActor :type Actor%20Object%20Reference))
  (|CallParentFunction OtherActor) ; This node is disabled and will not be called.\nDrag off pins to build functionality.
)

(event EventTick
  (params (DeltaSeconds :type Float%20%28single-precision%29))
  (|CallParentFunction DeltaSeconds) ; This node is disabled and will not be called.\nDrag off pins to build functionality.
)

(event EventPickedThisUp
  (params (Other%20Actor :type Actor%20Object%20Reference))
  ;[1 1 1 1 25] 게임모드의 시간이 올라가야하니까 게임모드에서 시간을 더할 변수(Time) 가져와서 원하는 더하기 값을 클램프로 미니맥스값을 지정해주고 다시 타임값에 set(적용)한다    타임업 이벤트가 발생하면 실행된다. 이벤트비긴플레이에 연결이 안되어 있을시 실행 오류가 뜨니 연결에 주의하자
  ;;[1 1 1 1 20] 픽디스업이벤트 발생시 타임업을 실행한다
  (CallFunction|TimeUp Other%20Actor))

(event EventBeginPlay
  ;[1 1 1 1 25] 게임모드의 시간이 올라가야하니까 게임모드에서 시간을 더할 변수(Time) 가져와서 원하는 더하기 값을 클램프로 미니맥스값을 지정해주고 다시 타임값에 set(적용)한다    타임업 이벤트가 발생하면 실행된다. 이벤트비긴플레이에 연결이 안되어 있을시 실행 오류가 뜨니 연결에 주의하자
  ;;[1 1 1] 비긴플레이에 게임모드레퍼런스를 가져와서 쓸 수 있게 하는 노드
  (bind _asbp_gm (Utilities|Casting|CastToBP_GM (Game|GetGameMode)))
  (Variables|Default|SetBP_GMTime _asbp_gm))

(fn ConstructionScript
  (|CallParentFunction))