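; BP_Inventory is an actor that demonstrates a simple item inventory holding a gun and a sword.
; On BeginPlay it spawns BP_Gun and BP_Sword at its own transform and adds both to the Items array.
; It then loops over Items and calls Use on each, so every item is triggered once at startup through a shared call.
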(event EventBeginPlay
  (bind _returnvalue (Game|SpawnActorfromClass "/Game/BluePrint/SaveGames/BP_Gun.BP_Gun_C" (Transformation|GetActorTransform) "Undefined" "MultiplyWithRoot" 0 0))
  (Utilities|Array|Add (Variables|Default|GetItems) _returnvalue)
  (bind _returnvalue_2 (Game|SpawnActorfromClass "/Game/BluePrint/SaveGames/BP_Sword.BP_Sword_C" (Transformation|GetActorTransform) "Undefined" "MultiplyWithRoot" 0 0))
  (Utilities|Array|Add (Variables|Default|GetItems) _returnvalue_2)
  (for _array_element (Variables|Default|GetItems)
    (Default|Use _array_element)))

(fn ConstructionScript)